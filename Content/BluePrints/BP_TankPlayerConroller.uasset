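; Player controller for the tank that drives the health bar HUD and shows the game-over screen.
; BeginPlay finds the tank pawn and, after a short delay, shows an animated ProgressBarHealth widget.
; Tick feeds the pawn's HealthComponent values to the bar, or flags death and zeroes it once the pawn is invalid.
; A delayed polling loop watches that flag, then swaps all widgets for the GameOver widget.
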(event `self.ReceiveBeginPlay`
  (`|ExecutionSequence`
    (:`then_0`
      (bind _returnvalue (`|CreateWidget` "/Game/BluePrints/Widget/ProgressBarHealth.ProgressBarHealth_C"))
      (bind _output_get (set `self.ProgressBarWidget` _returnvalue))
      (`KismetSystemLibrary.Delay` 1.9)
      (`UserWidget.AddToViewport` _output_get 0)
      (`/Game/BluePrints/Widget/ProgressBarHealth.PlayAnimPB` _output_get)
      (`KismetSystemLibrary.Delay` 0.1 :!label _label)
      (if (`self.Die Tank`)
        (`self.GameOverCustom`)
        (else
          (goto _label))))
    (:`then_1`
      (bind _returnvalue_2 (`GameplayStatics.GetActorOfClass` "/Game/BluePrints/bp_TankPawn.bp_TankPawn_C"))
      (set `self.Tank Pawn` _returnvalue_2))))

(event `self.ReceiveTick`
  (params (DeltaSeconds :type "Float (single-precision)"))
  (bind _healthcomponent (`TankPawn.HealthComponent` (`self.Tank Pawn`)))
  (`|ExecutionSequence`
    (:`then_0`
      (if (`KismetSystemLibrary.IsValid` (`self.Tank Pawn`))
        (`/Game/BluePrints/Widget/ProgressBarHealth.UpdateHeath` (`self.ProgressBarWidget`) (`HealthComponent.CurrentHealth` _healthcomponent) (`HealthComponent.MaxHealth` _healthcomponent))
        (else
          (set `self.Die Tank` true)
          (`/Game/BluePrints/Widget/ProgressBarHealth.UpdateHeath` (`self.ProgressBarWidget`) 0.0 0.0))))))

(event `GameOverCustom`
  (`WidgetLayoutLibrary.RemoveAllWidgets`)
  (bind _returnvalue (`|CreateWidget` "/Game/BluePrints/Widget/GameOver.GameOver_C"))
  (`UserWidget.AddToViewport` _returnvalue 0))

(fn `UserConstructionScript`)